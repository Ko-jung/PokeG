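; Test 2D character that walks on the world Y/Z plane with flipbook animations for four facing directions.
; IA_Move offsets the actor by raw input without sweep or delta-time scaling.
; GetDirection maps single-axis input to a facing, with no explicit diagonal case, and a change swaps the flipbook from the MoveDirect map.
; When input completes, the IdleDirect map supplies the idle flipbook for the last direction.
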(event `EnhancedInput|/Game/Character/Input/IA_Move`
  (params (ActionValue :type "Vector2D Structure") (ElapsedSeconds :type "Float (double-precision)") (TriggeredSeconds :type "Float (double-precision)") (InputAction :type "InputAction Object Reference" :default "/Game/Character/Input/IA_Move.IA_Move"))
  (:`Triggered`
    (`|ExecutionSequence`
      (:`then_0`
        (bind _resultdirection (`self.GetDirection` ActionValue_X ActionValue_Y))
        (if (not (== _resultdirection (`KismetMathLibrary.Conv_ByteToInt` (`self.Direction`))))
          (bind _output_get (set `self.Direction` _resultdirection))
          (`PaperFlipbookComponent.SetFlipbook` (`self.PaperFlipbook`) (`BlueprintMapLibrary.Map_Find` (`self.MoveDirect`) _output_get))))
      (:`then_1`
        (`self.K2_AddActorWorldOffset` (`KismetMathLibrary.MakeVector` 0.0 0.0 ActionValue_Y))
        (`self.K2_AddActorWorldOffset` (`KismetMathLibrary.MakeVector` 0.0 (* ActionValue_X -1.0))))))
  (:`Completed`
    (`PaperFlipbookComponent.SetFlipbook` (`self.PaperFlipbook`) (`BlueprintMapLibrary.Map_Find` (`self.IdleDirect`) (`self.Direction`)))))

(fn `GetDirection`
  (params (InputX :type "Float (double-precision)") (InputY :type "Float (double-precision)"))
  (returns (ResultDirection :type "EDirection Enum"))
  (`|ExecutionSequence`
    (:`then_0`
      (if (`KismetMathLibrary.NearlyEqual_FloatFloat` InputX)
        (if (> InputY 0.0)
          (return "Up")
          (else
            (return "Down")))))
    (:`then_1`
      (if (`KismetMathLibrary.NearlyEqual_FloatFloat` 0.0 InputY)
        (if (> InputX 0.0)
          (return "Right")
          (else
            (return "Left")))))
    (:`then_2`
      (if true
        _))))

(fn `UserConstructionScript`)